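; KLAC_DummyPayLoad is a placeholder payload that stands in for the payload bonus and effect logic alongside fairing and engine parts.
; SetAndActivateBonus and TryActivateEffect only print the class name, function name and bonus numbers they receive to screen as debug text.
; TryActivateEffect always returns true, the fairing and engine references go unused, and BeginPlay and Tick are disabled.
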(event EventBeginPlay
  (|CallParentFunction) ; このノードは無効になっているため呼び出せません。\n機能をビルドするにはピンをドラッグしてください。
)

(event EventTick
  (params (DeltaSeconds :type Float%20%28single-precision%29))
  (|CallParentFunction DeltaSeconds) ; このノードは無効になっているため呼び出せません。\n機能をビルドするにはピンをドラッグしてください。
)

(fn SetandActivateBonus
  (params (n_bonus :type Integer) (FairingPtr :type KLAC%20Fairing%20Base%20Object%20Reference%20%28by%20ref%29) (EnginePtr :type KLAC%20Engine%20Base%20Object%20Reference%20%28by%20ref%29))
  (Development|PrintString (Utilities|String|Append (Utilities|String|Append "class: " (Variables|Default|GetName) "; func SetAndActivateBonus") (Utilities|String|Append "; n_bonus: " (Utilities|String|ToString(Integer) n_bonus))) true true "(R=0.069704,G=1.000000,B=0.132436,A=1.000000)" 1e+01)
  (return))

(fn TryActivateEffect
  (params (n_fairing_bonus :type Integer) (n_payload_bonus :type Integer) (n_engine_bonus :type Integer) (FairingPtr :type KLAC%20Fairing%20Base%20Object%20Reference%20%28by%20ref%29) (EnginePtr :type KLAC%20Engine%20Base%20Object%20Reference%20%28by%20ref%29))
  (Development|PrintString (Utilities|String|Append (Utilities|String|Append "class: " (Variables|Default|GetName) "; func TryActivateEffect") (Utilities|String|Append "; n_fairing_bonus: " (Utilities|String|ToString(Integer) n_fairing_bonus)) (Utilities|String|Append "; n_payload_bonus: " (Utilities|String|ToString(Integer) n_payload_bonus)) (Utilities|String|Append "; n_engine_bonus: " (Utilities|String|ToString(Integer) n_engine_bonus))) true true "(R=0.069704,G=1.000000,B=0.132436,A=1.000000)" 1e+01)
  (return true))