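; KLAC_FairingBase is a base Blueprint that makes a flight direction wander over time.
; UpdateDirection continuously pitches the forward vector around the right vector at a per-second deviation rate, returning both updated vectors.
; At each fixed span it rolls the right vector around forward by a random angle from CalcDeviationAngleXY, carrying leftover time via modulo.
; Tick is empty, so callers drive updates; ResetToNextFlight clears the timer.
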(event EventBeginPlay
  (Variables|Default|SetTimeForSwitchDirection 0.0))

(event EventTick
  (params (DeltaSeconds :type Float%20%28single-precision%29)))

(fn UpdateDirection
  (params (InForwardVector :type Vector) (InRightVector :type Vector) (DeltaSecond :type Float%20%28single-precision%29))
  (LocalVariables|SetRight InRightVector)
  ;[1 1 1] 時間の更新
  (bind _output_get (Variables|Default|SetTimeForSwitchDirection (+ DeltaSecond (Variables|Default|GetTimeForSwitchDirection))))
  ;[1 1 1] 推進方向の切り替えタイミングの判定
  (if (<= (Variables|Define|GetDirectionChangeSpan) _output_get)
    ;[1 1 1] 時間のリセット
    (Variables|Default|SetTimeForSwitchDirection (Math|Float|%(Float) (Variables|Default|GetTimeForSwitchDirection) (Variables|Define|GetDirectionChangeSpan)))
    ;[1 1 1] 進行方向の更新
    (LocalVariables|SetRight (Math|Vector|RotateVectorAroundAxis InRightVector (Math|Conversions|ToFloat(Integer) (CallFunction|CalcDeviationAngleXY)) InForwardVector)))
  (return (Math|Vector|RotateVectorAroundAxis InForwardVector (* (Variables|Define|GetDeviationAnglePerSecond) DeltaSecond) (LocalVariables|GetRight)) (LocalVariables|GetRight)))

(fn CalcDeviationAngleXY
  (return (Math|Random|RandomInteger 360)))

(fn ResettoNextFlight
  (Variables|Default|SetTimeForSwitchDirection 0.0))