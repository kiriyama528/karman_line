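; Base payload part of a rocket, with a height-based score and a bonus effect tied to its linked fairing and engine.
; TryActivateEffect requires both linked parts and a CanActivateBonus pass before calling BonusEffect; default hooks pass height through, always allow, and do nothing.
; SetAndActivateBonus, not called here, rescales part weights exponentially by bonus count, though engine BaseWeight is derived from BasePower.
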(event EventBeginPlay)

(event EventTick
  (params (DeltaSeconds :type Float%20%28single-precision%29)))

(fn CalcScore
  (params (Height :type Float%20%28single-precision%29))
  (return Height))

(fn TryActivateEffect
  (params (n_fairing_bonus :type Integer) (n_payload_bonus :type Integer) (n_engine_bonus :type Integer) (FairingPtr :type KLAC%20Fairing%20Base%20Object%20Reference%20%28by%20ref%29) (EnginePtr :type KLAC%20Engine%20Base%20Object%20Reference%20%28by%20ref%29))
  (Utilities|FlowControl|Sequence
    (:then_0
      (bind _returnvalue (CallFunction|IsLinkedOtherParts FairingPtr EnginePtr))
      (if (not _returnvalue)
        (return false)))
    (:then_1
      (bind _can_activate (CallFunction|CanActivateBonus n_fairing_bonus n_payload_bonus n_engine_bonus))
      (if (not _can_activate)
        (return false)))
    (:then_2
      (CallFunction|BonusEffect n_fairing_bonus n_payload_bonus n_engine_bonus FairingPtr EnginePtr)
      (return true))))

(fn CanActivateBonus
  (params (n_fairing_bonus :type Integer) (n_payload_bonus :type Integer) (n_engine_bonus :type Integer))
  (return true))

(fn IsLinkedOtherParts
  (params (FairingPtr :type KLAC%20Fairing%20Base%20Object%20Reference%20%28by%20ref%29) (NewParam :type KLAC%20Engine%20Base%20Object%20Reference%20%28by%20ref%29))
  (return (and (Utilities|IsValid FairingPtr) (Utilities|IsValid NewParam))))

(fn BonusEffect
  (params (n_fairing_bonus :type Integer) (n_payload_bonus :type Integer) (n_engine_bonus :type Integer) (FairingPtr :type KLAC%20Fairing%20Base%20Object%20Reference%20%28by%20ref%29) (EnginePtr :type KLAC%20Engine%20Base%20Object%20Reference%20%28by%20ref%29)))

(fn SetandActivateBonus
  (params (n_bonus :type Integer) (FairingPtr :type KLAC%20Fairing%20Base%20Object%20Reference%20%28by%20ref%29) (EnginePtr :type KLAC%20Engine%20Base%20Object%20Reference%20%28by%20ref%29))
  ;[1 1 1] ペイロードに対して
  (Variables|Define|SetWeight (|(init*(power((1.000000-BONUS_RATE_),N_BONUS_))) (Variables|Define|GetWeight) (Math|Conversions|ToFloat(Integer) n_bonus) (Variables|Define|GetBONUS_RATE)))
  ;[1 1 1] フェアリングに対して
  (Variables|/Game/Blueprints/Fairings/KLAC_FairingBase.KLAC_FairingBase_C|SetWeight FairingPtr (|(init*(power((1.000000-BONUS_RATE_),N_BONUS_))) (Variables|/Game/Blueprints/Fairings/KLAC_FairingBase.KLAC_FairingBase_C|GetWeight FairingPtr) (Math|Conversions|ToFloat(Integer) n_bonus) (Variables|Define|GetBONUS_RATE)))
  ;[1 1 1] フェアリングに対して
  (Variables|/Game/Blueprints/Engines/KLAC_EngineBase.KLAC_EngineBase_C|SetBaseWeight EnginePtr (|(init*(power((1.000000-BONUS_RATE_),N_BONUS_))) (Variables|/Game/Blueprints/Engines/KLAC_EngineBase.KLAC_EngineBase_C|GetBasePower EnginePtr) (Math|Conversions|ToFloat(Integer) n_bonus) (Variables|Define|GetBONUS_RATE))))

(fn Print
  (Development|PrintString (Utilities|String|Append (Variables|Define|GetName) "; Weight : " (Utilities|String|ToString(Float) (Variables|Define|GetWeight))) true true "(R=0.024942,G=1.000000,B=0.198302,A=1.000000)" 1e+01))