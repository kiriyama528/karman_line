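; Zigzag fairing Blueprint that overrides UpdateDirection to alternate a flight direction between left and right.
; It accumulates delta time and flips FlightLeft each time DirectionChangeSpan elapses, carrying the remainder over.
; It returns a fixed Z-up vector rolled by plus or minus DeviationAnglePerSecond, unscaled by delta time.
; The incoming forward vector and parent implementation are unused.
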(event EventBeginPlay)

(event EventTick
  (params (DeltaSeconds :type Float%20%28single-precision%29)))

(fn UpdateDirection
  (params (InForwardVector :type Vector :default "0, 0, 0") (DeltaSecond :type Float%20%28single-precision%29))
  ;[1 1 1] 時間の更新
  (bind _output_get (Variables|Default|SetSpendTimeForSwitchDirection (+ DeltaSecond (Variables|Default|GetSpendTimeForSwitchDirection))))
  ;[1 1 1] 推進方向の切り替えタイミングの判定
  (if (<= (Variables|Default|GetDirectionChangeSpan) _output_get)
    ;[1 1 1] 時間のリセット
    (Variables|Default|SetSpendTimeForSwitchDirection (Math|Float|%(Float) (Variables|Default|GetSpendTimeForSwitchDirection) (Variables|Default|GetDirectionChangeSpan)))
    (Variables|ティック|Setflight_left (not (Variables|ティック|Getflight_left))))
  (return (Math|Vector|RotateVector "0, 0,1.000000" (Math|Rotator|MakeRotator (* (Variables|Default|GetDeviationAnglePerSecond) (Math|Float|SelectFloat 1.0 -1.0 (Variables|ティック|Getflight_left))) 0.0 0.0))))