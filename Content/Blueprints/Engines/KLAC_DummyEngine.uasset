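; KLAC_DummyEngine is a placeholder engine Blueprint with stub bonus handling and no active BeginPlay or Tick logic.
; Set and Activate Bonus prints a debug message with the class label, function name and count of engine bonuses received.
; It applies none of the bonuses and always returns zero Power and zero Weight.
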(event EventBeginPlay
  (|CallParentFunction) ; このノードは無効になっているため呼び出せません。\n機能をビルドするにはピンをドラッグしてください。
)

(event EventTick
  (params (DeltaSeconds :type Float%20%28single-precision%29))
  (|CallParentFunction DeltaSeconds) ; このノードは無効になっているため呼び出せません。\n機能をビルドするにはピンをドラッグしてください。
)

(fn SetandActivateBonus
  (params (EngineBonusList :type Array%20of%20KL%20Struct%20Engine%20Bonus%20Base%20Structures))
  (Development|PrintString (Utilities|String|Append (Utilities|String|Append "class: " (Variables|Default|GetName) "; func SetAndActivateBonus") (Utilities|String|Append "; n_bonus: " (Utilities|String|ToString(Integer) (Utilities|Array|Length EngineBonusList)))) true true "(R=0.069704,G=1.000000,B=0.132436,A=1.000000)" 1e+01)
  (return 0.0 0.0))