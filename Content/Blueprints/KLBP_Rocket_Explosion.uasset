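; Player rocket actor built from swappable Engine, Fairing, PayLoad and Body parts, launched once all are set and part bonuses are applied.
; Tick integrates engine thrust over total weight, fairing steering and gravity into velocity, then sweeps the actor along it, optionally warp-scaled, and turns it to face travel.
; Durability from the Body drains over time until explosion is triggered.
; A looping timer samples locations for a flight log with peak altitude and speed.
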(event Custom|Launch
  (bind (_is_set_all_parts _error_message) (CallFunction|IsSetAllParts))
  (if _is_set_all_parts
    ;[1 1 1] ボーナスおよび能力の適用
    (CallFunction|ActivateBonus (Variables|Default|GetFairing) (Variables|Default|GetPayLoad) (Variables|Default|GetEngine) (Variables|Bonus|GetN%20Fairing%20Bonus) (Variables|Bonus|GetN%20Payload%20Bonus) (Variables|Bonus|GetEngineBonus))
    ;[1 1 1] 耐久値の設定
    (CallFunction|CalcandSetDurability)
    ;[1 1 1] ロケット始動
    (Actor|Tick|SetActorTickEnabled true)
    (Variables|ティック|SetisLaunch true)
    (else
      (Development|PrintString (Utilities|String|Append "Error:can not launch. :" _error_message) true true "(R=1.000000,G=0.101376,B=0.061575,A=1.000000)"))))

(event Custom|NotLaunch
  (Actor|Tick|SetActorTickEnabled false)
  ;[1 1 1] フライトログの記録停止
  (Utilities|Time|ClearandInvalidateTimerbyHandle (Variables|Default|GetLocationTimer))
  ;[1 1 1] フライトログに最後の場所を記録
  (Utilities|Array|Add (Variables|FlightLog|GetLocations) (/ (Transformation|GetActorLocation) 1e+02))
  (Variables|ティック|SetisLaunch false))

(event Custom|RecordFlightLocation
  ;[1 1 1] FlightLogの更新
  (Utilities|Array|Add (Variables|FlightLog|GetLocations) (/ (Transformation|GetActorLocation) 1e+02)))

(event Custom|EventSetEngineBonus
  (params (TargetEngineBonus :type Array%20of%20KL%20Struct%20Engine%20Bonus%20Base%20Structures))
  ;[1 1 1] TODO:Event?Function?
  (Variables|Bonus|SetEngineBonus TargetEngineBonus))

(event Custom|EventSetEngine
  (params (TargetEngine :type KLAC%20Engine%20Base%20Object%20Reference))
  ;[1 1 1] TODO:Event?Function?
  (CallFunction|SetEngineParts TargetEngine))

(event Custom|EventSetFairing
  (params (TargetFairing :type KLAC%20Fairing%20Base%20Object%20Reference))
  (CallFunction|SetFairingParts TargetFairing))

(event Custom|EventSetFairingBonus
  (params (n_fairing_bonus :type Integer))
  (Variables|Bonus|SetN%20Fairing%20Bonus n_fairing_bonus))

(event Custom|EventSetPayLoadBonus
  (params (n_payload_bonus :type Integer))
  (Variables|Bonus|SetN%20Payload%20Bonus n_payload_bonus))

(event Custom|EventSetPayLoad
  (params (TargetPayLoad :type KLAC%20Pay%20Load%20Base%20Object%20Reference))
  (CallFunction|SetPayLoadParts TargetPayLoad))

(event EventBeginPlay
  (Utilities|FlowControl|Sequence
    (:then_0
      (Variables|Initial|SetInitialPosition (Transformation|GetActorLocation))
      (Variables|Initial|SetInitialRotation (Transformation|GetActorRotation)))
    (:then_1
      ;[0.4616 0.2237 1] FlightLogの記録タイマー
      (bind _returnvalue (Utilities|Time|SetTimerbyEvent (delegate Custom|RecordFlightLocation) (Variables|FlightLog|GetScoreTimeSpan) true))
      (Variables|Default|SetLocationTimer _returnvalue))))

(event EventTick
  (params (DeltaSeconds :type Float%20%28single-precision%29))
  (bind _returnvalue (Transformation|GetActorLocation))
  (bind _returnvalue_2 (Transformation|GetActorLocation))
  (bind _returnvalue_3 (/ (.z _returnvalue_2) 1e+02))
  (Variables|Tick|SetDeltaSeconds DeltaSeconds)
  (if (Variables|ティック|GetisLaunch)
    (Utilities|FlowControl|Sequence
      (:then_0
        ;[1 1 1] 数値の更新
        (bind _power (Default|BurnandGetPower (Variables|Default|GetEngine) (Variables|Tick|GetDeltaSeconds)))
        (bind _totalweight (CallFunction|UpdateWeight))
        (bind _acceleration (CallFunction|UpdateAcceleration _power _totalweight))
        (bind _updatedforward (Default|UpdateDirection (Variables|Default|GetFairing) (Variables|ティック|GetEngineDirection) (Variables|Tick|GetDeltaSeconds)))
        (bind _output_get (Variables|ティック|SetEngineDirection _updatedforward))
        (bind _output_get_2 (Variables|ティック|SetEngineAccelerationVector (* _output_get _acceleration))))
      (:then_1
        ;[1 1 1] 加速度ベクトルの総和
        (bind _output_get_3 (Variables|ティック|SetTotalAccelerationVector (+ (Variables|ティック|GetEngineAccelerationVector) (Variables|Define|GetGravityAccelerationVector))))
        (Development|PrintString (Utilities|String|Append "Flying vector:" (Utilities|String|ToString(Vector) _output_get_3)) true false "(R=0.000000,G=0.660000,B=1.000000,A=1.000000)" 0.0))
      (:then_2
        ;[1 1 1] 移動速度の計算
        (bind _speedvector (CallFunction|UpdateSpeed (Variables|ティック|GetSpeedVector) (Variables|ティック|GetTotalAccelerationVector) (Variables|Tick|GetDeltaSeconds)))
        (bind _output_get_4 (Variables|ティック|SetSpeedVector _speedvector))
        ;[1 1 1] Result用のデータ
        (if (< (Variables|FlightLog|GetMaxSpeed) (Math|Vector|VectorLength _output_get_4))
          (Variables|FlightLog|SetMaxSpeed (Math|Vector|VectorLength (Variables|ティック|GetSpeedVector)))))
      (:then_3
        ;[1 1 1] 今Tickの移動量の計算とActorへの適用_単純ver
        (bind _centimeter (CallFunction|M2cmVec (* (Variables|ティック|GetSpeedVector) (Variables|Tick|GetDeltaSeconds))))
        (bind _aftermovevector (CallFunction|WarpifNeeded _centimeter))
        (Transformation|AddActorWorldOffset _aftermovevector true)
        (Development|PrintString (Utilities|String|ToString(Vector) (Variables|ティック|GetSpeedVector)) true false "(R=0.000000,G=0.660000,B=1.000000,A=1.000000)" 0.0)
        ;[1 1 1] ロケット機体の向きを修正
        (Transformation|SetActorRotation (Math|Rotator|MakeRotator (.Roll (Math|Rotator|BreakRotator (Math|Rotator|FindLookatRotation _returnvalue (+ _returnvalue (Variables|ティック|GetSpeedVector))))) (+ (.Pitch (Math|Rotator|BreakRotator (Math|Rotator|FindLookatRotation _returnvalue (+ _returnvalue (Variables|ティック|GetSpeedVector))))) -9e+01) (.Yaw (Math|Rotator|BreakRotator (Math|Rotator|FindLookatRotation _returnvalue (+ _returnvalue (Variables|ティック|GetSpeedVector))))))))
      (:then_4
        ;[1 1 1] 耐久を減らし、耐久切れならば爆発イベント発行
        (bind _output_get_5 (Variables|ティック|SetDurability (- (Variables|ティック|GetDurability) (Variables|Tick|GetDeltaSeconds))))
        (if (<= _output_get_5 0.0)
          (Default|CallOnExplosion)))
      (:then_5
        ;[1 1 1] FlightLogのためのデータ更新
        (Variables|ティック|SetTotalTime (+ (Variables|ティック|GetTotalTime) (Variables|Tick|GetDeltaSeconds)))
        (if (< (Variables|FlightLog|GetHighScore) _returnvalue_3)
          (Variables|FlightLog|SetHighScore _returnvalue_3)
          (Variables|FlightLog|SetHighScoreTime (Variables|ティック|GetTotalTime)))))))

(fn ConstructionScript)

(fn CalcStroke
  (params (V0 :type Float%20%28single-precision%29) (a :type Float%20%28single-precision%29) (t :type Float%20%28single-precision%29))
  (return (|((v0*t)+((((1.000000/2.000000)*a)*t)*t)) V0 t a)))

(fn M2cm
  (params (meter :type Float%20%28single-precision%29))
  (return (* 100 meter)))

(fn M2cmVec
  (params (meter :type Vector))
  (return (* meter 100)))

(fn UpdateSpeed
  (params (v0 :type Vector) (a :type Vector) (time :type Float%20%28single-precision%29))
  (return (+ v0 (* a time))))

(fn UpdateAcceleration
  (params (F :type Float%20%28single-precision%29) (weight :type Float%20%28single-precision%29))
  (return (|(F/m) F weight)))

(fn ResettoNextFlight
  ;[1 0.2927 0.4026] 未メンテのため使わないようにしている
  (Development|PrintString "Error:KLBP_Rocket : Reset to Next Flight function is not maintenance." true true "(R=1.000000,G=0.071981,B=0.111783,A=1.000000)" 1e+01))

(fn UpdateWeight
  (bind _output_get (Variables|Default|SetTotalWeight (+ (Variables|/Game/Blueprints/Engines/KLAC_EngineBase.KLAC_EngineBase_C|GetWeight (Variables|Default|GetEngine)) (Variables|/Game/Blueprints/Fairings/KLAC_FairingBase.KLAC_FairingBase_C|GetWeight (Variables|Default|GetFairing)) (Variables|/Game/Blueprints/PayLoad/KLAC_PayLoadBase.KLAC_PayLoadBase_C|GetWeight (Variables|Default|GetPayLoad)))))
  (return _output_get))

(fn GetFlightLog
  (return (Utilities|Struct|MakeKLStruct_FlightLog (Variables|FlightLog|GetHighScore) (Variables|FlightLog|GetHighScoreTime) (Variables|FlightLog|GetScoreTimeSpan) (Variables|FlightLog|GetLocations) (Variables|Default|GetPayLoad) (Variables|Default|GetTotalWeight) (Variables|FlightLog|GetMaxSpeed))))

(fn SetFairingParts
  (params (InputPin :type KLAC%20Fairing%20Base%20Object%20Reference))
  ;[1 1 1] すでにセットされているものは破棄
  (Utilities|IsValid (Variables|Default|GetFairing)
    (:Is%20Valid
      (Components|DestroyComponent (Variables|Default|GetFairing)))
    (:Is%20Not%20Valid
      _))
  (Variables|Default|SetFairing InputPin)
  (Variables|ティック|SetEngineDirection (Variables|/Game/Blueprints/Fairings/KLAC_FairingBase.KLAC_FairingBase_C|GetInitialDirection (Variables|Default|GetFairing))))

(fn SetEngineParts
  (params (InputPin :type KLAC%20Engine%20Base%20Object%20Reference))
  ;[1 1 1] すでにセットされているものは破棄
  (Utilities|IsValid (Variables|Default|GetEngine)
    (:Is%20Valid
      (Components|DestroyComponent (Variables|Default|GetEngine)))
    (:Is%20Not%20Valid
      _))
  (Variables|Default|SetEngine InputPin))

(fn IsSetAllParts
  (bind _engine (Variables|Default|GetEngine))
  (bind _fairing (Variables|Default|GetFairing))
  (bind _payload (Variables|Default|GetPayLoad))
  (bind _body (Variables|Default|GetBody))
  (bind _returnvalue (Utilities|IsValid _engine))
  (bind _returnvalue_2 (Utilities|IsValid _fairing))
  (bind _returnvalue_3 (Utilities|IsValid _body))
  (bind _returnvalue_4 (Utilities|IsValid _payload))
  (return (Math|Boolean|ANDBoolean _returnvalue _returnvalue_2 _returnvalue_4 _returnvalue_3) (Utilities|String|Append (Utilities|String|SelectString "Engine is not set." "" _returnvalue) (Utilities|String|SelectString "Fairing is not set." "" _returnvalue_2) (Utilities|String|SelectString "PayLoad is not set." "" _returnvalue_4) (Utilities|String|SelectString "Body is not set." "" _returnvalue_3))))

(fn WarpifNeeded
  (params (MoveVector :type Vector))
  (if (Variables|SpecialEffect|GetCanWarp)
    (return (* MoveVector (Variables|Define|GetWarpRate)) (Variables|SpecialEffect|GetCanWarp))
    (else
      (return MoveVector (Variables|SpecialEffect|GetCanWarp)))))

(fn ActivateBonus
  (params (FairingPtr :type KLAC%20Fairing%20Base%20Object%20Reference%20%28by%20ref%29) (PayLoadPtr :type KLAC%20Pay%20Load%20Base%20Object%20Reference%20%28by%20ref%29) (EnginePtr :type KLAC%20Engine%20Base%20Object%20Reference%20%28by%20ref%29) (n_fairing_bonus :type Integer) (n_payload_bonus :type Integer) (engine_bonus_list :type Array%20of%20KL%20Struct%20Engine%20Bonus%20Base%20Structures))
  ;[1 0.03073 0.02078] 将来的には、これがEngineBonusListと置き換わるイメージ
  (LocalVariables|Setn_engine_bonus (Utilities|Array|Length engine_bonus_list))
  (Default|TryActivateEffect PayLoadPtr n_fairing_bonus n_payload_bonus (LocalVariables|Getn_engine_bonus) FairingPtr EnginePtr)
  (Default|SetandActivateBonus PayLoadPtr n_payload_bonus FairingPtr EnginePtr)
  (Default|SetandActivateBonus FairingPtr n_fairing_bonus)
  (Default|SetandActivateBonus EnginePtr engine_bonus_list))

(fn SetPayLoadParts
  (params (TargetPayLoad :type KLAC%20Pay%20Load%20Base%20Object%20Reference))
  ;[1 1 1] すでにセットされているものは破棄
  (Utilities|IsValid (Variables|Default|GetPayLoad)
    (:Is%20Valid
      (Components|DestroyComponent (Variables|Default|GetPayLoad)))
    (:Is%20Not%20Valid
      _))
  (Variables|Default|SetPayLoad TargetPayLoad))

(fn SetSpecialFlagifNeeded
  ;[1 1 1] ワープを有効化するか
  (bind _asklac_warp_pay_load (Utilities|Casting|CastToKLAC_WarpPayLoad (Variables|Default|GetPayLoad))
    (:then
      (bind _can_activate (Default|CanActivateBonus _asklac_warp_pay_load (Variables|Bonus|GetN%20Fairing%20Bonus) (Variables|Bonus|GetN%20Payload%20Bonus) (Utilities|Array|Length (Variables|Bonus|GetEngineBonus))))
      (Variables|SpecialEffect|SetCanWarp _can_activate))
    (:CastFailed
      (Variables|SpecialEffect|SetCanWarp false))))

(fn CalcandSetDurability
  (bind _output_get (Variables|ティック|SetDurability (Variables|/Game/Blueprints/Body/KLAC_BodyBase.KLAC_BodyBase_C|GetDurability (Variables|Default|GetBody))))
  (return _output_get))

(fn SetBodyParts
  (params (TargetBody :type KLAC%20Body%20Base%20Object%20Reference))
  ;[1 1 1] すでにセットされているものは破棄
  (Utilities|IsValid (Variables|Default|GetBody)
    (:Is%20Valid
      (Components|DestroyComponent (Variables|Default|GetBody)))
    (:Is%20Not%20Valid
      _))
  (Variables|Default|SetBody TargetBody))