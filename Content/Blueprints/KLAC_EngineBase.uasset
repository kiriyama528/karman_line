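; KLAC_EngineBase is a base engine that supplies power and carries a weight for flights, with a limited running time.
; Each GetPower call adds burn time to the running total, then returns Power while under the maximum, otherwise zero.
; SetAndActivateBonus rebuilds Power and Weight from their base values plus an array of bonuses.
; ResetToNextFlight clears the running time between flights.
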(event EventBeginPlay
  (Variables|デフォルト|SetPower (Variables|Define|GetBasePower))
  (Variables|デフォルト|SetWeight (Variables|Define|GetBaseWeight)))

(event EventTick
  (params (DeltaSeconds :type Float%20%28single-precision%29)))

(fn IsRunning
  (return (< (Variables|Default|GetRunningTime) (Variables|define|GetMaxRunningTime))))

(fn GetPower
  (params (AddBurnTime :type Float%20%28single-precision%29))
  ;[1 0.05208 0.05208] fix me : update running time is after burning ?
  (bind _output_get (Variables|Default|SetRunningTime (+ AddBurnTime (Variables|Default|GetRunningTime))))
  (bind _isrunning (CallFunction|IsRunning))
  (if _isrunning
    (return (Variables|デフォルト|GetPower))
    (else
      (return 0.0))))

(fn ResettoNextFlight
  (Variables|Default|SetRunningTime 0.0))

(fn SetandActivateBonus
  (params (NewParam :type Array%20of%20KL%20Struct%20Engine%20Bonus%20Base%20Structures))
  ;[1 1 1] 初期値に戻す
  (Variables|デフォルト|SetPower (Variables|Define|GetBasePower))
  (Variables|デフォルト|SetWeight (Variables|Define|GetBaseWeight))
  (bind _output_get (Variables|Default|SetBonus NewParam))
  (for _array_element _output_get
    (Variables|デフォルト|SetPower (+ (Variables|デフォルト|GetPower) (.PowerBonus (Utilities|Struct|BreakKLStruct_EngineBonusBase _array_element))))
    (Variables|デフォルト|SetWeight (+ (Variables|デフォルト|GetWeight) (.WeightBonus (Utilities|Struct|BreakKLStruct_EngineBonusBase _array_element)))))
  (return (Variables|デフォルト|GetPower) (Variables|デフォルト|GetWeight)))