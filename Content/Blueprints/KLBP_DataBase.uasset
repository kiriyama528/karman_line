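; Per-map parts database for rocket building, holding the selectable engines, fairings and engine bonuses.
; On BeginPlay it adds engine and fairing components into arrays, sizes a reveal list covering every engine-fairing pairing and fills the bonus list.
; Scroll functions cycle the current indices with wraparound, and getters return the selected part and name.
; HUD getters return normalized power, deviation and weight, or zeros until that pairing is revealed.
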(event EventBeginPlay
  (Utilities|FlowControl|Sequence
    (:then_0
      ;[1 1 1] 本マップにおけるロケットエンジンリストを生成
      (Utilities|FlowControl|Sequence
        (:then_0
          (bind _returnvalue (AddComponent|AddKLACEngineBase))
          (bind _returnvalue_2 (AddComponent|AddKLACRichEngine))
          (bind _returnvalue_3 (AddComponent|AddKLACShortEngine))
          (Variables|Default|SetEngineIndex 0))
        (:then_1
          (Variables|Default|SetEngines (Utilities|Array|MakeArray _returnvalue _returnvalue_2 _returnvalue_3)))))
    (:then_1
      ;[1 1 1] 本マップにおけるフェアリングリストを生成
      (Utilities|FlowControl|Sequence
        (:then_0
          (bind _returnvalue_4 (AddComponent|AddKLACBasicFairing))
          (bind _returnvalue_5 (AddComponent|AddKLACZigzagFairing))
          (bind _returnvalue_6 (AddComponent|AddKLACStraightFairing))
          (bind _returnvalue_7 (AddComponent|AddKLACLeaningFairing))
          (Variables|Default|SetFairingIndex 0))
        (:then_1
          (Variables|Default|SetFairings (Utilities|Array|MakeArray _returnvalue_4 _returnvalue_5 _returnvalue_6 _returnvalue_7)))))
    (:then_2
      (Utilities|Array|Resize (Variables|Default|GetRevealList) (* (Utilities|Array|Length (Variables|Default|GetEngines)) (Utilities|Array|Length (Variables|Default|GetFairings)))))
    (:then_3
      (Variables|Default|SetEngineBonus (Utilities|Array|MakeArray (Utilities|Struct|MakeKLStruct_EngineBonusBase "PowerBonus" 1e+01 0.0) (Utilities|Struct|MakeKLStruct_EngineBonusBase "WeightBonus" 0.0 1e+01))))))

(fn ConstructionScript)

(fn GetFairing
  (bind _fairings (Variables|Default|GetFairings))
  (bind _fairingindex (Variables|Default|GetFairingIndex))
  (bind _output (Utilities|Array|Get(acopy) _fairings _fairingindex))
  (return _output (Variables|/Game/Blueprints/Fairings/KLAC_FairingBase.KLAC_FairingBase_C|GetName _output)))

(fn GetEngine
  (bind _engines (Variables|Default|GetEngines))
  (bind _engineindex (Variables|Default|GetEngineIndex))
  (bind _output (Utilities|Array|Get(acopy) _engines _engineindex))
  (return _output (Variables|/Game/Blueprints/Engines/KLAC_EngineBase.KLAC_EngineBase_C|GetName _output)))

(fn ScrollNextEngine
  (bind _returnvalue (CallFunction|NextEngineIdx (Variables|Default|GetEngines)))
  (bind _output_get (Variables|Default|SetEngineIndex _returnvalue))
  (return _output_get))

(fn ScrollBeforeEngine
  (bind _returnvalue (CallFunction|BeforeEngineIdx (Variables|Default|GetEngines)))
  (bind _output_get (Variables|Default|SetEngineIndex _returnvalue))
  (return _output_get))

(fn ScrollNextFairing
  (bind _returnvalue (CallFunction|NextFairingIdx (Variables|Default|GetFairings)))
  (bind _output_get (Variables|Default|SetFairingIndex _returnvalue))
  (return _output_get))

(fn ScrollBeforeFairing
  (bind _returnvalue (CallFunction|BeforeFairingIdx (Variables|Default|GetFairings)))
  (bind _output_get (Variables|Default|SetFairingIndex _returnvalue))
  (return _output_get))

(fn ResettoNextFlight
  ;[1 1 1] Do Nothing
)

(fn RevealParameters
  (Utilities|Array|SetArrayElem (Variables|Default|GetRevealList) (CallFunction|CalcIndex (Variables|Default|GetFairingIndex) (Variables|Default|GetEngineIndex)) true))

(fn GetParamsforHUD
  (bind _engines (Variables|Default|GetEngines))
  (bind _engineindex (Variables|Default|GetEngineIndex))
  (bind _fairings (Variables|Default|GetFairings))
  (bind _fairingindex (Variables|Default|GetFairingIndex))
  (bind _output (Utilities|Array|Get(acopy) _engines _engineindex))
  (bind _output_2 (Utilities|Array|Get(acopy) _fairings _fairingindex))
  (if (Utilities|Array|Get(acopy) (Variables|Default|GetRevealList) (CallFunction|CalcIndex (Variables|Default|GetFairingIndex) (Variables|Default|GetEngineIndex)))
    ;[1 1 1] Revealed
    (return (/ (Variables|/Game/Blueprints/Engines/KLAC_EngineBase.KLAC_EngineBase_C|GetPower _output) 1e+05) (/ (Variables|/Game/Blueprints/Fairings/KLAC_FairingBase.KLAC_FairingBase_C|GetDeviationAnglePerSecond _output_2) 9e+01) (/ (+ (Variables|/Game/Blueprints/Engines/KLAC_EngineBase.KLAC_EngineBase_C|GetWeight _output) (Variables|/Game/Blueprints/Fairings/KLAC_FairingBase.KLAC_FairingBase_C|GetWeight _output_2) 0.0) 1e+04))
    (else
      ;[1 1 1] UnRevealed
      (return 0.0 0.0 0.0))))

(fn CalcIndex
  (params (FairingIndex :type Integer) (EngineIndex :type Integer))
  (return (+ (* FairingIndex (Utilities|Array|Length (Variables|Default|GetEngines))) EngineIndex)))

(fn RevealParametersAll
  ;[1 1 1] 未公開が1つでもあれば
  (if (Utilities|Array|ContainsItem (Variables|Default|GetRevealList) false)
    (for _index (range 0 (Utilities|Array|Length (Variables|Default|GetRevealList)))
      (Utilities|Array|SetArrayElem (Variables|Default|GetRevealList) _index true))))

(fn GetEngineBonus
  (bind _enginebonus (Variables|Default|GetEngineBonus))
  (bind _engineindex (Variables|Default|GetEngineIndex))
  (bind _returnvalue (Utilities|Array|Length _enginebonus))
  (bind _returnvalue_2 (Math|Integer|%(Integer) _engineindex _returnvalue))
  (bind _output (Utilities|Array|Get(acopy) _enginebonus _returnvalue_2))
  (return _output (.Name (Utilities|Struct|BreakKLStruct_EngineBonusBase _output))))

(fn BeforeEngineIdx
  (params (TargetArray :type Array%20of%20KLAC%20Engine%20Base%20Object%20References))
  (bind _engineindex (Variables|Default|GetEngineIndex))
  (bind _returnvalue (- _engineindex 1))
  (return (Math|Integer|SelectInt (- (Utilities|Array|Length TargetArray) 1) _returnvalue (< _returnvalue 0))))

(fn BeforeFairingIdx
  (params (TargetArray :type Array%20of%20KLAC%20Fairing%20Base%20Object%20References))
  (bind _fairingindex (Variables|Default|GetFairingIndex))
  (bind _returnvalue (- _fairingindex 1))
  (return (Math|Integer|SelectInt (- (Utilities|Array|Length TargetArray) 1) _returnvalue (< _returnvalue 0))))

(fn NextEngineIdx
  (params (TargetEngineArray :type Array%20of%20KLAC%20Engine%20Base%20Object%20References))
  (return (Math|Integer|%(Integer) (+ (Variables|Default|GetEngineIndex) 1) (Utilities|Array|Length TargetEngineArray))))

(fn NextFairingIdx
  (params (TargtFairingArray :type Array%20of%20KLAC%20Fairing%20Base%20Object%20References))
  (return (Math|Integer|%(Integer) (+ (Variables|Default|GetFairingIndex) 1) (Utilities|Array|Length TargtFairingArray))))