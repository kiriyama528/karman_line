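; Debug fairing Blueprint that overrides UpdateDirection to compute a forward direction from one of three test motion patterns.
; Dragon mode tilts the up vector once by the deviation angle, then sweeps it around yaw on a looping timer, tracing a cone every DirectionChangeSpan.
; Leaning mode returns a fixed tilt from vertical; otherwise the incoming vector rolls continuously, scaled by delta time.
; The parent's UpdateDirection is never called.
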(event EventBeginPlay
  (|CallParentFunction) ; このノードは無効になっているため呼び出せません。\n機能をビルドするにはピンをドラッグしてください。
)

(event EventTick
  (params (DeltaSeconds :type Float%20%28single-precision%29))
  (|CallParentFunction DeltaSeconds) ; このノードは無効になっているため呼び出せません。\n機能をビルドするにはピンをドラッグしてください。
)

(fn UpdateDirection
  (params (InForwardVector :type Vector :default "0, 0, 0") (DeltaSecond :type Float%20%28single-precision%29))
  (if (Variables|Default|GetIsDragon)
    (if (Variables|Default|GetIs%20First%20Update%20Direction)
      ;[1 1 1] 初回は初期値を代入
      (Variables|Default|SetInitialForwardDirection (Math|Vector|RotateVector "0, 0,1.000000" (Math|Rotator|MakeRotator (Variables|Default|GetDeviationAnglePerSecond) 0.0 0.0)))
      (Variables|Default|SetIs%20First%20Update%20Direction false))
    (Variables|Default|SetSpendTimeForSwitchDirection (|((total+delta)%change_span) (Variables|Default|GetSpendTimeForSwitchDirection) DeltaSecond (Variables|Default|GetDirectionChangeSpan)))
    (return (Math|Vector|RotateVector (Variables|Default|GetInitialForwardDirection) (Math|Rotator|MakeRotator 0.0 0.0 (* 360 (/ (Variables|Default|GetSpendTimeForSwitchDirection) (Variables|Default|GetDirectionChangeSpan))))))
    (elif (Variables|Default|GetIsLeaning)
      (return (Math|Vector|RotateVector "0, 0,1.000000" (Math|Rotator|MakeRotator (Variables|Default|GetDeviationAnglePerSecond) 0.0 0.0)))
      (else
        (return (Math|Vector|RotateVector InForwardVector (Math|Rotator|MakeRotator (* (Variables|Default|GetDeviationAnglePerSecond) DeltaSecond) 0.0 0.0)))))))