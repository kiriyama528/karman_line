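; Camera actor that follows a target actor with an independent tracking mode for each world axis.
; BeginPlay records the starting offset from the target, and Tick repositions the actor each frame while the target is valid.
; CalcLocation resolves each axis by its mode: match the target, keep the initial offset, or stay fixed.
; SetTargetActor swaps the target without recalculating the stored offset.
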(event EventBeginPlay
  (Variables|Default|SetDitanceFromTarget (- (Transformation|GetActorLocation) (Transformation|GetActorLocation (Variables|Default|GetTarget)))))

(event EventTick
  (params (DeltaSeconds :type Float%20%28single-precision%29))
  (bind _returnvalue (Transformation|GetActorLocation))
  (bind _ditancefromtarget (Variables|Default|GetDitanceFromTarget))
  (bind _target (Variables|Default|GetTarget))
  (bind _returnvalue_2 (Transformation|GetActorLocation _target))
  (if (Utilities|IsValid (Variables|Default|GetTarget))
    (Transformation|SetActorLocation (Math|Vector|MakeVector (CallFunction|CalcLocation (.x _returnvalue_2) (.x _returnvalue) (Variables|Default|GetTrackingX) (.x _ditancefromtarget)) (CallFunction|CalcLocation (.y _returnvalue_2) (.y _returnvalue) (Variables|Default|GetTrackingY) (.y _ditancefromtarget)) (CallFunction|CalcLocation (.z _returnvalue_2) (.z _returnvalue) (Variables|Default|GetTrackingZ) (.z _ditancefromtarget))) false false)))

(fn ConstructionScript)

(fn SetTargetActor
  (params (Target :type Actor%20Object%20Reference))
  (Variables|Default|SetTarget Target))

(fn CalcLocation
  (params (TargetLocation :type Float%20%28single-precision%29) (MyLocation :type Float%20%28single-precision%29) (TrackingParam :type KLEnum_TrackingParam%20Enum :default "NewEnumerator0") (DistanceFromTarget :type Float%20%28single-precision%29))
  (switch Utilities|FlowControl|Switch|SwitchonKLEnum_TrackingParam TrackingParam
    (:NewEnumerator0
      (return TargetLocation))
    (:NewEnumerator1
      (return (+ TargetLocation DistanceFromTarget)))
    (:NewEnumerator2
      (return MyLocation))))