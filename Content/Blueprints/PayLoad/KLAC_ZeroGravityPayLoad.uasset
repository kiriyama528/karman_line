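; KLAC_ZeroGravityPayLoad is a payload Blueprint for what appears to be a rocket part system, granting a zero-gravity set bonus.
; It overrides CanActivateBonus to activate once the payload bonus count reaches a threshold, ignoring fairing and engine counts.
; Its BonusEffect override zeroes the payload's own weight, the fairing's weight and the engine's base weight, without calling the parent implementations.
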(event EventBeginPlay
  (|CallParentFunction) ; このノードは無効になっているため呼び出せません。\n機能をビルドするにはピンをドラッグしてください。
)

(event EventTick
  (params (DeltaSeconds :type Float%20%28single-precision%29))
  (|CallParentFunction DeltaSeconds) ; このノードは無効になっているため呼び出せません。\n機能をビルドするにはピンをドラッグしてください。
)

(fn CanActivateBonus
  (params (n_fairing_bonus :type Integer) (n_payload_bonus :type Integer) (n_engine_bonus :type Integer))
  (return (<= 7 n_payload_bonus)))

(fn BonusEffect
  (params (n_fairing_bonus :type Integer) (n_payload_bonus :type Integer) (n_engine_bonus :type Integer) (FairingPtr :type KLAC%20Fairing%20Base%20Object%20Reference%20%28by%20ref%29) (EnginePtr :type KLAC%20Engine%20Base%20Object%20Reference%20%28by%20ref%29))
  (Variables|Default|SetWeight 0.0)
  (Variables|/Game/Blueprints/Fairings/KLAC_FairingBase.KLAC_FairingBase_C|SetWeight FairingPtr 0.0)
  (Variables|/Game/Blueprints/Engines/KLAC_EngineBase.KLAC_EngineBase_C|SetBaseWeight EnginePtr 0.0)
  (return))