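; Payload Blueprint for a Long Vernier part that grants a bonus extending the engine's running time.
; It overrides CanActivateBonus to activate only when the engine bonus count reaches a fixed threshold, ignoring fairing and payload counts.
; BonusEffect then adds a time constant to the engine's MaxRunningTime.
; The event graph holds only disabled BeginPlay and Tick stubs.
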(event EventBeginPlay
  (|CallParentFunction) ; このノードは無効になっているため呼び出せません。\n機能をビルドするにはピンをドラッグしてください。
)

(event EventTick
  (params (DeltaSeconds :type Float%20%28single-precision%29))
  (|CallParentFunction DeltaSeconds) ; このノードは無効になっているため呼び出せません。\n機能をビルドするにはピンをドラッグしてください。
)

(fn CanActivateBonus
  (params (n_fairing_bonus :type Integer) (n_payload_bonus :type Integer) (n_engine_bonus :type Integer))
  (return (<= 4 n_engine_bonus)))

(fn BonusEffect
  (params (n_fairing_bonus :type Integer) (n_payload_bonus :type Integer) (n_engine_bonus :type Integer) (FairingPtr :type KLAC%20Fairing%20Base%20Object%20Reference%20%28by%20ref%29) (EnginePtr :type KLAC%20Engine%20Base%20Object%20Reference%20%28by%20ref%29))
  (Variables|/Game/Blueprints/Engines/KLAC_EngineBase.KLAC_EngineBase_C|SetMaxRunningTime EnginePtr (+ (LocalVariables|GetBONUS_ADD_TIME) (Variables|/Game/Blueprints/Engines/KLAC_EngineBase.KLAC_EngineBase_C|GetMaxRunningTime EnginePtr))))