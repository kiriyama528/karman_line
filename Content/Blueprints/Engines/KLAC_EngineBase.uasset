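; Base engine Blueprint that models thrust power, weight and a limited burn time per flight.
; Power and Weight start from base values; SetAndActivateBonus resets them, then compounds each bonus multiplicatively, raising power and reducing weight.
; GetPower adds the burn time before checking the limit, returning Power while running and zero afterwards; a fix-me note questions that order.
; ResetToNextFlight clears the running time, and Print shows the base stats on screen.
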(event EventBeginPlay
  (Variables|ティック|SetPower (Variables|Define|GetBasePower))
  (Variables|ティック|SetWeight (Variables|Define|GetBaseWeight)))

(event EventTick
  (params (DeltaSeconds :type Float%20%28single-precision%29)))

(fn IsRunning
  (return (< (Variables|Tick|GetRunningTime) (Variables|define|GetMaxRunningTime))))

(fn GetPower
  (params (AddBurnTime :type Float%20%28single-precision%29))
  ;[1 0.05208 0.05208] fix me : update running time is after burning ?
  (bind _output_get (Variables|Tick|SetRunningTime (+ AddBurnTime (Variables|Tick|GetRunningTime))))
  (bind _isrunning (CallFunction|IsRunning))
  (if _isrunning
    (return (Variables|ティック|GetPower))
    (else
      (return 0.0))))

(fn ResettoNextFlight
  (Variables|Tick|SetRunningTime 0.0))

(fn SetandActivateBonus
  (params (EngineBonusList :type Array%20of%20KL%20Struct%20Engine%20Bonus%20Base%20Structures))
  ;[1 1 1] 初期値に戻す
  (Variables|ティック|SetPower (Variables|Define|GetBasePower))
  (Variables|ティック|SetWeight (Variables|Define|GetBaseWeight))
  (bind _output_get (Variables|ティック|SetBonus EngineBonusList))
  (for _array_element _output_get
    (Variables|ティック|SetPower (* (Variables|ティック|GetPower) (+ 1.0 (.PowerBonus (Utilities|Struct|BreakKLStruct_EngineBonusBase _array_element)))))
    (Variables|ティック|SetWeight (* (Variables|ティック|GetWeight) (- 1.0 (.WeightBonus (Utilities|Struct|BreakKLStruct_EngineBonusBase _array_element))))))
  (return (Variables|ティック|GetPower) (Variables|ティック|GetWeight)))

(fn Print
  (Development|PrintString (Utilities|String|Append (Variables|Define|GetName) " ; Base Power: " (Utilities|String|ToString(Float) (Variables|Define|GetBasePower)) "; Base Weight: " (Utilities|String|ToString(Float) (Variables|Define|GetBaseWeight)) "; Max Running Time: " (Utilities|String|ToString(Float) (Variables|define|GetMaxRunningTime))) true true "(R=0.024942,G=1.000000,B=0.198302,A=1.000000)" 1e+01))