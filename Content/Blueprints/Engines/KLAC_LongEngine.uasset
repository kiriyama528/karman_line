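; KLAC_LongEngine is an engine Blueprint whose bonus extends how long the engine can run.
; It overrides Set and Activate Bonus to add the length of the engine bonus list to MaxRunningTime, then returns Power and Weight unchanged.
; The parent bonus call is left unconnected, and the BeginPlay and Tick events are disabled placeholders.
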(event EventBeginPlay
  (|CallParentFunction) ; このノードは無効になっているため呼び出せません。\n機能をビルドするにはピンをドラッグしてください。
)

(event EventTick
  (params (DeltaSeconds :type Float%20%28single-precision%29))
  (|CallParentFunction DeltaSeconds) ; このノードは無効になっているため呼び出せません。\n機能をビルドするにはピンをドラッグしてください。
)

(fn SetandActivateBonus
  (params (EngineBonusList :type Array%20of%20KL%20Struct%20Engine%20Bonus%20Base%20Structures))
  (Variables|Default|SetMaxRunningTime (+ (Variables|Default|GetMaxRunningTime) (Math|Conversions|ToFloat(Integer) (Utilities|Array|Length EngineBonusList))))
  (return (Variables|Default|GetPower) (Variables|Default|GetWeight)))