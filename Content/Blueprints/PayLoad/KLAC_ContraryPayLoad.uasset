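; KLAC_ContraryPayLoad is a payload Blueprint whose bonus inverts the engine's power and weight.
; CanActivateBonus enables it once the payload bonus count is at least four, ignoring fairing and engine counts.
; BonusEffect computes both values before assigning: weight becomes one tenth of the old power, and power becomes ten times the old weight.
; The fairing is untouched, and neither override calls its parent.
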(event EventBeginPlay
  (|CallParentFunction) ; このノードは無効になっているため呼び出せません。\n機能をビルドするにはピンをドラッグしてください。
)

(event EventTick
  (params (DeltaSeconds :type Float%20%28single-precision%29))
  (|CallParentFunction DeltaSeconds) ; このノードは無効になっているため呼び出せません。\n機能をビルドするにはピンをドラッグしてください。
)

(fn CanActivateBonus
  (params (n_fairing_bonus :type Integer) (n_payload_bonus :type Integer) (n_engine_bonus :type Integer))
  (return (<= 4 n_payload_bonus)))

(fn BonusEffect
  (params (n_fairing_bonus :type Integer) (n_payload_bonus :type Integer) (n_engine_bonus :type Integer) (FairingPtr :type KLAC%20Fairing%20Base%20Object%20Reference%20%28by%20ref%29) (EnginePtr :type KLAC%20Engine%20Base%20Object%20Reference%20%28by%20ref%29))
  ;[1 1 1] 値の準備
  (LocalVariables|SetAfterWeight (|(power*(1000.000000/10000)) (Variables|/Game/Blueprints/Engines/KLAC_EngineBase.KLAC_EngineBase_C|GetPower EnginePtr)))
  (LocalVariables|SetAfterPower (|(_weight*(10000.000000/1000)) (Variables|/Game/Blueprints/Engines/KLAC_EngineBase.KLAC_EngineBase_C|GetWeight EnginePtr)))
  ;[1 1 1] 代入
  (Variables|/Game/Blueprints/Engines/KLAC_EngineBase.KLAC_EngineBase_C|SetPower EnginePtr (LocalVariables|GetAfterPower))
  (Variables|/Game/Blueprints/Engines/KLAC_EngineBase.KLAC_EngineBase_C|SetWeight EnginePtr (LocalVariables|GetAfterWeight))
  (return))