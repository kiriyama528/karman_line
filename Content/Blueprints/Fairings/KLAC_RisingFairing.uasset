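; KLAC_RisingFairing is a fairing Blueprint that overrides its parent's direction update to swing the initial direction over time.
; UpdateDirection accumulates elapsed time and unrotates InitialDirection by a roll growing linearly to a 90-degree cap over DirectionChangeSpan.
; SetAndActivateBonus shortens that span exponentially by (1 − BonusRate)^NBonus, quickening the turn, and returns DeviationAnglePerSecond unchanged.
; Neither override calls its parent; BeginPlay and Tick are disabled stubs.
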(event EventBeginPlay
  (|CallParentFunction) ; このノードは無効になっているため呼び出せません。\n機能をビルドするにはピンをドラッグしてください。
)

(event EventTick
  (params (DeltaSeconds :type Float%20%28single-precision%29))
  (|CallParentFunction DeltaSeconds) ; このノードは無効になっているため呼び出せません。\n機能をビルドするにはピンをドラッグしてください。
)

(fn UpdateDirection
  (params (InForwardVector :type Vector :default "0, 0, 0") (DeltaSecond :type Float%20%28single-precision%29))
  ;[1 1 1] 時間の更新
  (Variables|Default|SetSpendTimeForSwitchDirection (+ DeltaSecond (Variables|Default|GetSpendTimeForSwitchDirection)))
  (return (Math|Vector|UnrotateVector (Variables|Default|GetInitialDirection) (Math|Rotator|MakeRotator (Math|Float|Min(Float) (|((90.000000/end_time)*spend_time) (Variables|Default|GetDirectionChangeSpan) (Variables|Default|GetSpendTimeForSwitchDirection)) 9e+01) 0.0 0.0))))

(fn SetandActivateBonus
  (params (n_bonus :type Integer))
  (Variables|Default|SetDirectionChangeSpan (|(Span*(power((1.000000-bonus_rate),pow))) (Variables|Define|GetBonusRate) (Math|Conversions|ToFloat(Integer) n_bonus) (Variables|Default|GetDirectionChangeSpan)))
  (return (Variables|Default|GetDeviationAnglePerSecond)))