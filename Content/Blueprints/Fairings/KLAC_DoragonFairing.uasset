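; Doragon fairing Blueprint that overrides UpdateDirection to supply its own rotating forward direction.
; The first update seeds ForwardDirection from InitialDirection, pitched by DeviationAnglePerSecond.
; Every update then yaws it by an angle derived from DirectionChangeSpan and delta time, with delta time in the divisor.
; The input vectors are ignored, the parent implementation is not called, and the returned right vector is zero.
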(event EventBeginPlay
  (|CallParentFunction) ; このノードは無効になっているため呼び出せません。\n機能をビルドするにはピンをドラッグしてください。
)

(event EventTick
  (params (DeltaSeconds :type Float%20%28single-precision%29))
  (|CallParentFunction DeltaSeconds) ; このノードは無効になっているため呼び出せません。\n機能をビルドするにはピンをドラッグしてください。
)

(fn UpdateDirection
  (params (InForwardVector :type Vector :default "0, 0, 0") (InRightVector :type Vector :default "0, 0, 0") (DeltaSecond :type Float%20%28single-precision%29))
  (if (Variables|ティック|GetIsFirstUpdateDirection)
    ;[1 1 1] 初回は初期値を代入
    (Variables|Tick|SetForwardDirection (Math|Vector|RotateVector (Variables|Default|GetInitialDirection) (Math|Rotator|MakeRotator 0.0 (Variables|Default|GetDeviationAnglePerSecond) 0.0)))
    (Variables|ティック|SetIsFirstUpdateDirection false))
  (bind _output_get (Variables|Tick|SetForwardDirection (Math|Vector|RotateVector (Variables|Tick|GetForwardDirection) (Math|Rotator|MakeRotator 0.0 0.0 (/ 3.6e+02 (/ DeltaSecond (Variables|Default|GetDirectionChangeSpan)))))))
  (return _output_get "0, 0, 0"))