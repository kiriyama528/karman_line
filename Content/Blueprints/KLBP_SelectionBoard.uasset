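; Selection board for choosing rocket parts, keeping scrollable lists of engines and fairings with a current index for each.
; BeginPlay copies the source arrays and shuffles them unless a debug flag disables it.
; Scroll functions move the indices, while PushPop functions swap parts by adding any valid returned item and removing the indexed one.
; HUD stats are normalized and zeroed for unrevealed combinations, with fairing values read from the unshuffled source array.
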(event EventBeginPlay
  (|CallParentFunction)
  (Utilities|FlowControl|Sequence
    (:then_0
      (bind _output_get (Variables|Default|SetEngineList (Variables|Default|GetEngines)))
      (if (not (Variables|Default|GetInvalidShuffleForDebug))
        (Utilities|Array|Shuffle _output_get)))
    (:then_1
      (bind _output_get_2 (Variables|Default|SetFairingList (Variables|Default|GetFairings)))
      (if (not (Variables|Default|GetInvalidShuffleForDebug))
        (Utilities|Array|Shuffle _output_get_2)))))

(event Collision|EventActorBeginOverlap
  (params (OtherActor :type Actor%20Object%20Reference)))

(event EventTick
  (params (DeltaSeconds :type Float%20%28single-precision%29)))

(fn ConstructionScript
  (|CallParentFunction))

(fn GetEngine
  (bind _enginelist (Variables|Default|GetEngineList))
  (bind _engineindex (Variables|Default|GetEngineIndex))
  (bind _output (Utilities|Array|Get(acopy) _enginelist _engineindex))
  (bind _returnvalue (Utilities|GetDisplayName _output))
  ;[1 0.0625 0.0625] for debug
  (Development|PrintString _returnvalue)
  (return _output _returnvalue))

(fn GetFairing
  (bind _engineindex (Variables|Default|GetEngineIndex))
  (bind _fairinglist (Variables|Default|GetFairingList))
  (bind _output (Utilities|Array|Get(acopy) _fairinglist _engineindex))
  (return _output (Utilities|GetDisplayName _output)))

(fn ScrollBeforeEngine
  (bind _returnvalue (CallFunction|BeforeEngineIdx (Variables|Default|GetEngineList)))
  (bind _output_get (Variables|Default|SetEngineIndex _returnvalue))
  (return _output_get))

(fn ScrollBeforeFairing
  (bind _returnvalue (CallFunction|BeforeFairingIdx (Variables|Default|GetFairingList)))
  (bind _output_get (Variables|Default|SetFairingIndex _returnvalue))
  (return _output_get))

(fn ScrollNextEngine
  (bind _returnvalue (CallFunction|NextEngineIdx (Variables|Default|GetEngineList)))
  (bind _output_get (Variables|Default|SetEngineIndex _returnvalue))
  (return _output_get))

(fn ScrollNextFairing
  (bind _returnvalue (CallFunction|NextFairingIdx (Variables|Default|GetFairingList)))
  (bind _output_get (Variables|Default|SetFairingIndex _returnvalue))
  (return _output_get))

(fn GetParamsforHUD
  (bind _engineindex (Variables|Default|GetEngineIndex))
  (bind _enginelist (Variables|Default|GetEngineList))
  (bind _fairings (Variables|Default|GetFairings))
  (bind _fairingindex (Variables|Default|GetFairingIndex))
  (bind _output (Utilities|Array|Get(acopy) _enginelist _engineindex))
  (bind _output_2 (Utilities|Array|Get(acopy) _fairings _fairingindex))
  (if (Utilities|Array|Get(acopy) (Variables|Default|GetRevealList) (CallFunction|CalcIndex (Variables|Default|GetFairingIndex) (Variables|Default|GetEngineIndex)))
    ;[1 1 1] Revealed
    (return (/ (Variables|/Game/Blueprints/Engines/KLAC_EngineBase.KLAC_EngineBase_C|GetPower _output) 1e+05) (/ (Variables|/Game/Blueprints/Fairings/KLAC_FairingBase.KLAC_FairingBase_C|GetDeviationAnglePerSecond _output_2) 9e+01) (/ (+ (Variables|/Game/Blueprints/Engines/KLAC_EngineBase.KLAC_EngineBase_C|GetWeight _output) (Variables|/Game/Blueprints/Fairings/KLAC_FairingBase.KLAC_FairingBase_C|GetWeight _output_2) 0.0) 1e+04))
    (else
      ;[1 1 1] UnRevealed
      (return 0.0 0.0 0.0))))

(fn PushEngine
  (params (Engine :type KLAC%20Engine%20Base%20Object%20Reference))
  (bind _returnvalue (Utilities|Array|Add (Variables|Default|GetEngineList) Engine))
  (return _returnvalue))

(fn PushFairing
  (params (Fairing :type KLAC%20Fairing%20Base%20Object%20Reference))
  (bind _returnvalue (Utilities|Array|Add (Variables|Default|GetFairingList) Fairing))
  (return _returnvalue))

(fn PopEngine
  (bind _enginelist (Variables|Default|GetEngineList))
  (LocalVariables|Setresult (Utilities|Array|Get(acopy) _enginelist (Variables|Default|GetEngineIndex)))
  (Utilities|Array|RemoveIndex _enginelist (Variables|Default|GetEngineIndex))
  (Variables|Default|SetEngineIndex (Math|Integer|%(Integer) (Variables|Default|GetEngineIndex) (Utilities|Array|Length (Variables|Default|GetEngineList))))
  ;[1 0.0625 0.0625] for debug
  (Development|PrintString (Utilities|GetDisplayName (LocalVariables|Getresult)))
  (return (LocalVariables|Getresult) (Utilities|GetDisplayName (LocalVariables|Getresult))))

(fn PopFairing
  (bind _returnvalue (Utilities|GetDisplayName 0))
  (bind _fairinglist (Variables|Default|GetFairingList))
  (LocalVariables|Setresult (Utilities|Array|Get(acopy) _fairinglist (Variables|Default|GetFairingIndex)))
  (Utilities|Array|RemoveIndex _fairinglist (Variables|Default|GetFairingIndex))
  (Variables|Default|SetFairingIndex (Math|Integer|%(Integer) (Variables|Default|GetFairingIndex) (Utilities|Array|Length (Variables|Default|GetFairingList))))
  ;[1 0.0625 0.0625] for debug
  (Development|PrintString _returnvalue)
  (return (LocalVariables|Getresult) _returnvalue))

(fn PushPopEngine
  (params (PushedItem :type KLAC%20Engine%20Base%20Object%20Reference))
  (Utilities|IsValid PushedItem
    (:Is%20Valid
      ;[1 1 1] 入れ替え対象があるとき
      (CallFunction|PushEngine PushedItem))
    (:Is%20Not%20Valid
      _))
  (bind _engine (CallFunction|PopEngine))
  (return _engine))

(fn PushPopFairing
  (params (PushedItem :type KLAC%20Fairing%20Base%20Object%20Reference))
  (Utilities|IsValid PushedItem
    (:Is%20Valid
      ;[1 1 1] 入れ替え対象があるとき
      (CallFunction|PushFairing PushedItem))
    (:Is%20Not%20Valid
      _))
  (bind _fairing (CallFunction|PopFairing))
  (return _fairing))