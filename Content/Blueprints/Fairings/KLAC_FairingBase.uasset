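; Base fairing component that computes how a flight's forward direction drifts over time.
; UpdateDirection bends forward around the right vector at a per-second deviation rate, periodically rolling that right vector around forward by a random angle to change drift direction.
; BeginPlay derives an orthogonal axis from the initial direction, ResetToNextFlight clears the switch timer, and SetAndActivateBonus compounds reductions to the deviation rate.
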(event EventBeginPlay
  (Variables|Tick|SetSpendTimeForSwitchDirection 0.0)
  (Variables|Define|SetInitialDirection (Math|Vector|Normalize (Variables|Define|GetInitialDirection)))
  (Variables|ティック|SetOrthogonalDirection (Math|Vector|GetRightVector (Math|Rotator|MakeRotfromZ (Math|Vector|Normalize (Variables|Define|GetInitialDirection))))))

(event EventTick
  (params (DeltaSeconds :type Float%20%28single-precision%29)))

(fn UpdateDirection
  (params (InForwardVector :type Vector) (InRightVector :type Vector) (DeltaSecond :type Float%20%28single-precision%29))
  (LocalVariables|SetRight InRightVector)
  ;[1 1 1] 時間の更新
  (bind _output_get (Variables|Tick|SetSpendTimeForSwitchDirection (+ DeltaSecond (Variables|Tick|GetSpendTimeForSwitchDirection))))
  ;[1 1 1] 推進方向の切り替えタイミングの判定
  (if (<= (Variables|Define|GetDirectionChangeSpan) _output_get)
    ;[1 1 1] 時間のリセット
    (Variables|Tick|SetSpendTimeForSwitchDirection (Math|Float|%(Float) (Variables|Tick|GetSpendTimeForSwitchDirection) (Variables|Define|GetDirectionChangeSpan)))
    ;[1 1 1] 進行方向の更新
    (LocalVariables|SetRight (Math|Vector|RotateVectorAroundAxis InRightVector (Math|Conversions|ToFloat(Integer) (CallFunction|CalcDeviationAngleXY)) InForwardVector)))
  (return (Math|Vector|RotateVectorAroundAxis InForwardVector (* (Variables|Define|GetDeviationAnglePerSecond) DeltaSecond) (LocalVariables|GetRight)) (LocalVariables|GetRight)))

(fn CalcDeviationAngleXY
  (return (Math|Random|RandomInteger 360)))

(fn ResettoNextFlight
  (Variables|Tick|SetSpendTimeForSwitchDirection 0.0))

(fn SetandActivateBonus
  (params (n_bonus :type Integer))
  (for _index (range 0 n_bonus)
    (Variables|Define|SetDeviationAnglePerSecond (* (Variables|Define|GetDeviationAnglePerSecond) (- 1.0 (LocalVariables|GetBONUS_RATE)))))
  (return (Variables|Define|GetDeviationAnglePerSecond)))